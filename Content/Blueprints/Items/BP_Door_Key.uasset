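; BP_Door_Key is a key pickup that unlocks doors with a matching number when the player touches it.
; On sphere overlap with BP_Player, it searches all BP_Door actors for a DoorNumber equal to its KeyNumber.
; For each match it clears DoorLocked, calls UnlockDoor and destroys the key, so an unmatched key stays in place.
; The construction script displays KeyNumber on a text render component.
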(event `self.Sphere.OnComponentBeginOverlap`
  (params (OverlappedComponent :type "PrimitiveComponent Object Reference") (OtherActor :type "Actor Object Reference") (OtherComp :type "PrimitiveComponent Object Reference") (OtherBodyIndex :type Integer) (bFromSweep :type Boolean) (SweepResult :type "HitResult Structure (by ref)"))
  (cast `/Game/Blueprints/BP_Player` OtherActor)
  (bind _outactors (`GameplayStatics.GetAllActorsOfClass` "/Game/Blueprints/Items/BP_Door.BP_Door_C"))
  (for _array_element _outactors
    (if (== (`/Game/Blueprints/Items/BP_Door.DoorNumber` _array_element) (`self.KeyNumber`))
      (set `/Game/Blueprints/Items/BP_Door.DoorLocked` false _array_element)
      (`/Game/Blueprints/Items/BP_Door.UnlockDoor` _array_element)
      (`self.K2_DestroyActor`))))

(fn `UserConstructionScript`
  (`TextRenderComponent.K2_SetText` (`self.TextRender`) (`KismetTextLibrary.Conv_IntToText` (`self.KeyNumber`))))