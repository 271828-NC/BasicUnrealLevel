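; BP_Door is a numbered 2D sprite door that the player opens with the Interact input unless it is locked.
; Overlapping its box enables input and prints a prompt, and leaving disables it.
; Interacting either prints a locked message or hides the sprite and disables its collision.
; The construction script sets the number label and lock-state sprite, while UnlockDoor only refreshes that sprite from DoorLocked without changing the flag.
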(event `self.Box.OnComponentBeginOverlap`
  (params (OverlappedComponent :type "PrimitiveComponent Object Reference") (OtherActor :type "Actor Object Reference") (OtherComp :type "PrimitiveComponent Object Reference") (OtherBodyIndex :type Integer) (bFromSweep :type Boolean) (SweepResult :type "HitResult Structure (by ref)"))
  (cast `/Game/Blueprints/BP_Player` OtherActor)
  (`self.EnableInput` (`GameplayStatics.GetPlayerController` 0))
  (`KismetSystemLibrary.PrintString` "Press E"))

(event `self.Box.OnComponentEndOverlap`
  (params (OverlappedComponent :type "PrimitiveComponent Object Reference") (OtherActor :type "Actor Object Reference") (OtherComp :type "PrimitiveComponent Object Reference") (OtherBodyIndex :type Integer))
  (cast `/Game/Blueprints/BP_Player` OtherActor)
  (`self.DisableInput` (`GameplayStatics.GetPlayerController` 0)))

(event `InputAction|Interact`
  (params (Key :type "Key Structure"))
  (bind _doorsprite (`self.DoorSprite`))
  (:`Pressed`
    (if (`self.DoorLocked`)
      (`KismetSystemLibrary.PrintString` "Door Locked")
      (else
        (`PrimitiveComponent.SetCollisionEnabled` _doorsprite "NoCollision")
        (`SceneComponent.SetVisibility` _doorsprite false false)))))

(event `UnlockDoor`
  (bind _doorsprite (`self.DoorSprite`))
  (if (`self.DoorLocked`)
    (`PaperSpriteComponent.SetSprite` _doorsprite "/Game/Sprites/UI/Healthbars/SimpleGameBars_Sprite_4.SimpleGameBars_Sprite_4")
    (else
      (`PaperSpriteComponent.SetSprite` _doorsprite "/Game/Sprites/UI/Healthbars/SimpleGameBars_Sprite_28.SimpleGameBars_Sprite_28"))))

(fn `UserConstructionScript`
  (bind _doorsprite (`self.DoorSprite`))
  (`TextRenderComponent.K2_SetText` (`self.TextRender`) (`KismetTextLibrary.Conv_IntToText` (`self.DoorNumber`)))
  (if (`self.DoorLocked`)
    (`PaperSpriteComponent.SetSprite` _doorsprite "/Game/Sprites/UI/Healthbars/SimpleGameBars_Sprite_4.SimpleGameBars_Sprite_4")
    (else
      (`PaperSpriteComponent.SetSprite` _doorsprite "/Game/Sprites/UI/Healthbars/SimpleGameBars_Sprite_28.SimpleGameBars_Sprite_28"))))