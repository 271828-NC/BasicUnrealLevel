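; BP_Goal is the level exit door, which completes the level when a BP_Player carrying the key overlaps its box trigger.
; On success it swaps the Paper2D sprite to the open door, plays a sound and shows WBP_LevelComplete with UI-only input and a visible cursor, then disables player movement.
; Without the key it only prints a "Key Required" message.
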(event `self.Box.OnComponentBeginOverlap`
  (params (OverlappedComponent :type "PrimitiveComponent Object Reference") (OtherActor :type "Actor Object Reference") (OtherComp :type "PrimitiveComponent Object Reference") (OtherBodyIndex :type Integer) (bFromSweep :type Boolean) (SweepResult :type "HitResult Structure (by ref)"))
  (bind _returnvalue (`GameplayStatics.GetPlayerController` 0))
  (bind _asbp_player (cast `/Game/Blueprints/BP_Player` OtherActor))
  (if (`/Game/Blueprints/BP_Player.HasKey?` _asbp_player)
    (`PaperSpriteComponent.SetSprite` (`self.PaperSprite`) "/Game/Sprites/Items/dark-wood-open_Sprite.dark-wood-open_Sprite")
    (`GameplayStatics.PlaySound2D` null 1.0 1.0 0.0 null null)
    (bind _returnvalue_2 (`|CreateWidget` "/Game/Blueprints/Widgets/WBP_LevelComplete.WBP_LevelComplete_C"))
    (`UserWidget.AddToViewport` _returnvalue_2 0)
    (`WidgetBlueprintLibrary.SetInputMode_UIOnlyEx` _returnvalue _returnvalue_2)
    (set `PlayerController.bShowMouseCursor` true _returnvalue)
    (`CharacterMovementComponent.DisableMovement` (`Character.CharacterMovement` _asbp_player))
    (else
      (`KismetSystemLibrary.PrintString` "Key Required"))))

(fn `UserConstructionScript`)