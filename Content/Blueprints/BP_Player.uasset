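; Player character for a 2D flipbook side-scroller, with run, sprint, optional double jump, coin counting and a HUD.
; Tick picks the flipbook from state and movement, and flips facing via control rotation from X velocity; attacking only blocks new input and changes animation.
; Capsule hits on BP_Simple_Enemy use hit direction to either stomp-damage and bounce, or knock back, hurt and flash the player red.
; Damage reduces clamped health, setting Dead at zero.
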(event `self.ReceiveBeginPlay`
  ;[1 1 1] Begin Play
  (bind _returnvalue (`|CreateWidget` "/Game/Blueprints/Widgets/WBP_Player_HUD.WBP_Player_HUD_C"))
  (bind _output_get (set `self.PlayerHud` _returnvalue))
  (`UserWidget.AddToViewport` _output_get 0))

(event `self.ReceiveTick`
  (params (DeltaSeconds :type "Float (single-precision)"))
  ;[1 1 1] Event Tick
  ;;[0.1647 1 0.7176] This Calls the animation event
  (`self.UpdateAnimation`)
  ;;[0.5569 0.4157 1] This calls the character rotation event
  (`self.UpdateRotation`)
  (`self.CheckOxygen`))

(event `UpdateRotation`
  ;[0.5569 0.4157 1] Rotation/Flip player
  (`/Engine/EditorBlueprintResources/StandardMacros.CompareFloat` 0.0 (.x (`self.GetVelocity`))
    (:`>`
      ;;[1 1 1] Rotate Player to face right
      (`Controller.SetControlRotation` (`GameplayStatics.GetPlayerController` 0) (`KismetMathLibrary.MakeRotator` 0.0 0.0 180.0)))
    (:`<`
      ;;[1 1 1] RotatePlayer to face left
      (`Controller.SetControlRotation` (`GameplayStatics.GetPlayerController` 0) (`KismetMathLibrary.MakeRotator` 0.0)))))

(event `CheckOxygen`)

(event `InputAxis|MoveRight`
  (params (AxisValue :type "Float (single-precision)"))
  ;[1 1 1] Movement
  (if (not (or (`self.bDead`) (`self.Attacking`)))
    (`self.AddMovementInput` (1.0 0.0 0.0) AxisValue)))

(event `InputAction|Jump`
  (params (Key :type "Key Structure"))
  ;[1 1 1] Jumping
  (:`Pressed`
    (if (not (or (`self.bDead`) (`self.Attacking`)))
      (`self.Jump`)
      ;;[1 1 1] Adds 1 to Jump Count
      (`/Engine/EditorBlueprintResources/StandardMacros.IncrementInt` (`self.JumpCount`))))
  (:`Released`
    (`self.StopJumping`)))

(event `self.OnLanded`
  (params (Hit :type "HitResult Structure (by ref)"))
  ;[1 1 1] Jumping
  ;;[1 1 1] Resets Jump Count when landing
  (set `self.JumpCount` 0))

(event `UpdateAnimation`
  ;[0.1647 1 0.7176] Animation Update
  (if (`self.bDead`)
    ;;[1 0 0.001733] Set Flipbook to Dead
    (`PaperFlipbookComponent.SetFlipbook` (`self.Sprite`) (`self.Dead Flipbook`))
    (elif (`self.IsHurt`)
      ;;[1 0 0.001733] Set Flipbook to Hurt
      (`PaperFlipbookComponent.SetFlipbook` (`self.Sprite`) (`self.Hurt Flipbook`))
      (elif (`NavMovementComponent.IsFalling` (`self.CharacterMovement`))
        ;;[1 1 1] Is the character going up or down? (Z Axis)
        (`/Engine/EditorBlueprintResources/StandardMacros.CompareFloat` (.z (`self.GetVelocity`))
          (:`>`
            ;;[1 1 1] Is it jump 1 or 2? (double jump)
            (if (> (`self.JumpCount`) 1)
              ;;[1 1 1] Set Flipbook to double jump
              (`PaperFlipbookComponent.SetFlipbook` (`self.Sprite`) (`self.Double Jump Flipbook`))
              (else
                ;;[1 1 1] Set Flipbook to jump
                (`PaperFlipbookComponent.SetFlipbook` (`self.Sprite`) (`self.Jump Flipbook`)))))
          (:`<`
            ;;[1 1 1] Set Flipbook to Falling
            (`PaperFlipbookComponent.SetFlipbook` (`self.Sprite`) (`self.Falling Flipbook`))))
        (elif (`self.Attacking`)
          ;;[1 1 1] Set Flipbook to Attack
          (`PaperFlipbookComponent.SetFlipbook` (`self.Sprite`) (`self.Attack Flipbook`))
          (elif (> (`KismetMathLibrary.VSize` (`self.GetVelocity`)) 0.0)
            ;;[1 1 1] Set Flipbook to Run
            (`PaperFlipbookComponent.SetFlipbook` (`self.Sprite`) (`self.Run Flipbook`))
            (else
              ;[1 1 1] Set Flipbook to Idle
              (`PaperFlipbookComponent.SetFlipbook` (`self.Sprite`) (`self.Idle Flipbook`)))))))))

(event `Key|LeftMouseButton`
  (params (Key :type "Key Structure"))
  ;[1 1 1] Attack
  (:`Pressed`
    (if (not (or (`self.bDead`) (`self.Attacking`)))
      (set `self.Attacking` true)))
  (:`Released`
    (set `self.Attacking` false)))

(event `InputAction|Sprint`
  (params (Key :type "Key Structure"))
  (bind _charactermovement (`self.CharacterMovement`))
  (:`Pressed`
    (if (`self.Can Sprint`)
      (set `CharacterMovementComponent.MaxWalkSpeed` (`self.SprintSpeed`) _charactermovement)))
  (:`Released`
    (set `CharacterMovementComponent.MaxWalkSpeed` (`self.WalkSpeed`) _charactermovement)))

(event `AddCoin`
  ;[1 1 1] Add Coin
  (bind _output_get (set `self.Coins` (+ (`self.Coins`) 1)))
  (`KismetSystemLibrary.PrintString` (`KismetStringLibrary.Conv_IntToString` _output_get)))

(event `Key|H`
  (params (Key :type "Key Structure"))
  ;[1 1 1] Debug
  ;;[1 1 1] Test Health
  (:`Pressed`
    (`GameplayStatics.ApplyDamage` self 25.0)))

(event `self.ReceiveAnyDamage`
  (params (Damage :type "Float (single-precision)") (DamageType :type "DamageType Object Reference") (InstigatedBy :type "Controller Object Reference") (DamageCauser :type "Actor Object Reference"))
  ;[0.6344 0.343 0.3655] Player Health
  ;;[1 1 1] Take damage amount from health and set it between 0 and 100
  (bind _output_get (set `self.Health` (`KismetMathLibrary.FClamp` (- (`self.Health`) Damage) 0.0 100.0)))
  (`KismetSystemLibrary.PrintString` (`KismetStringLibrary.Conv_DoubleToString` _output_get))
  (if (and (<= (`self.Health`) 0.0) (not (`self.bDead`)))
    (set `self.bDead` true)))

(event `Key|LeftShift`
  (params (Key :type "Key Structure"))
  (bind _charactermovement (`self.CharacterMovement`))
  ;[1 1 1] Sprint
  (:`Pressed`
    (set `CharacterMovementComponent.MaxWalkSpeed` 800.0 _charactermovement))
  (:`Released`
    (set `CharacterMovementComponent.MaxWalkSpeed` 400.0 _charactermovement)))

(event `self.CapsuleComponent.OnComponentHit`
  (params (HitComponent :type "PrimitiveComponent Object Reference") (OtherActor :type "Actor Object Reference") (OtherComp :type "PrimitiveComponent Object Reference") (NormalImpulse :type "Vector Structure") (Hit :type "HitResult Structure (by ref)"))
  ;[1 1 1] Enemy Interaction
  (bind _asbp_simple_enemy (cast `/Game/Blueprints/Enemys/BP_Simple_Enemy` OtherActor))
  (set `self.EnemyRef` _asbp_simple_enemy)
  (set `self.HitDirection` (`KismetMathLibrary.Normal` (- Hit_Location (`self.K2_GetActorLocation`)) 0.0))
  ;;[1 1 1] Check if hitting enemy from above
  (if (<= (.z (`self.HitDirection`)) -0.1)
    (set `MovementComponent.Velocity` (0.0 0.0 0.0) (`self.CharacterMovement`))
    (`MovementComponent.StopMovementImmediately` (`self.CharacterMovement`))
    (`CharacterMovementComponent.AddImpulse` (`self.CharacterMovement`) (0.0 0.0 500.0) true)
    ;;[1 1 1] Damage Enemy
    (`GameplayStatics.ApplyDamage` (`self.EnemyRef`) 100.0)
    (else
      (set `MovementComponent.Velocity` (0.0 0.0 0.0) (`self.CharacterMovement`))
      (`MovementComponent.StopMovementImmediately` (`self.CharacterMovement`))
      (`CharacterMovementComponent.AddImpulse` (`self.CharacterMovement`) (`KismetMathLibrary.MakeVector` (* (.x (`self.HitDirection`)) (* -1.0 300.0)) 0.0 300.0) true)
      ;;[1 1 1] Damage Self
      (`GameplayStatics.ApplyDamage` self 20.0)
      ;[1 1 1] player flashed red
      (set `self.IsHurt` true)
      (`PaperFlipbookComponent.SetSpriteColor` (`self.Sprite`) (struct :`R` 1.0 :`G` 0.027692 :`A` 1.0))
      (`KismetSystemLibrary.Delay` 0.5)
      (set `self.IsHurt` false)
      (`PaperFlipbookComponent.SetSpriteColor` (`self.Sprite`) (struct :`R` 1.0 :`G` 1.0 :`B` 1.0 :`A` 1.0)))))

(event `InputAction|Crouch`
  (params (Key :type "Key Structure"))
  ;[1 1 1] OLD CODE
)

(fn `UserConstructionScript`
  (`|ExecutionSequence`
    (:`then_0`
      (if (`self.Can Double Jump`)
        (set `self.JumpMaxCount` 2)
        (else
          (set `self.JumpMaxCount` 1))))
    (:`then_1`
      (set `self.JumpHoldTime` (`self.JumpHoldTime`)))
    (:`then_2`
      (set `CharacterMovementComponent.MaxWalkSpeed` (`self.WalkSpeed`) (`self.CharacterMovement`)))))