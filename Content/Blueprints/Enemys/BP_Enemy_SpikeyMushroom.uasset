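; Spikey mushroom enemy, a child Blueprint with a flipbook sprite that patrols back and forth along the X axis.
; It picks a random direction on BeginPlay, moves each tick while alive, and reverses on X-normal capsule hits with anything but the player.
; FlipSprite mirrors the sprite through its X scale.
; Parent overrides set the dying flipbook and destroy the actor on death.
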(event `self.ReceiveBeginPlay`
  (`parent.ReceiveBeginPlay`)
  ;[1 1 1] Randomly selects a direction
  (set `self.MoveRight` (`KismetMathLibrary.RandomBool`))
  ;[0.5569 0.4157 1] Flips the sprite based on direction (double click node to see function)
  (`self.FlipSprite`))

(event `self.ReceiveTick`
  (params (DeltaSeconds :type "Float (single-precision)"))
  ;[1 1 1] As a child bluprint, all parent code is also executed
  (`parent.ReceiveTick` DeltaSeconds)
  ;[1 1 1] Check enemy is not dead
  (if (not (`self.bDead`))
    ;[1 1 1] Add movement every tick
    (`self.AddMovementInput` (1.0 0.0 0.0) (select `bool` (`self.MoveRight`) :`false` -1.0 :`true` 1.0 :!type "Float (single-precision)"))))

(event `self.CapsuleComponent.OnComponentHit`
  (params (HitComponent :type "PrimitiveComponent Object Reference") (OtherActor :type "Actor Object Reference") (OtherComp :type "PrimitiveComponent Object Reference") (NormalImpulse :type "Vector Structure") (Hit :type "HitResult Structure (by ref)"))
  (if (!= OtherActor (`GameplayStatics.GetPlayerPawn` 0))
    (if (!= (.x Hit_Normal) 0.0)
      ;[1 1 1] Toggle boolean
      (set `self.MoveRight` (not (`self.MoveRight`)))
      ;[0.5569 0.4157 1] Flips the sprite based on direction (double click node to see function)
      (`self.FlipSprite`))))

(fn `DeathAnimation`
  (`PaperFlipbookComponent.SetFlipbook` (`self.Sprite`) "/Game/Textures/myTextures/Demon_Dying1.Demon_Dying1")
  (`parent.DeathAnimation`))

(fn `EnemyDied`
  (`parent.EnemyDied`)
  (`KismetSystemLibrary.PrintString` "Enemy Destroyed")
  (`self.K2_DestroyActor`))

(fn `FlipSprite`
  (bind (_returnvalue_x _returnvalue_y _returnvalue_z) (`KismetMathLibrary.BreakVector` (`SceneComponent.K2_GetComponentScale` (`self.Sprite`))))
  (`SceneComponent.SetWorldScale3D` (`self.Sprite`) (`KismetMathLibrary.MakeVector` (* (select `bool` (`self.MoveRight`) :`false` -1.0 :`true` 1.0 :!type "Float (single-precision)") (`KismetMathLibrary.Abs` _returnvalue_x)) _returnvalue_y _returnvalue_z)))

(fn `UserConstructionScript`
  (`parent.UserConstructionScript`))