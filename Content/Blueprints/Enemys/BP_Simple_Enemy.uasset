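; BP_Simple_Enemy is a 2D flipbook enemy that patrols along the X axis until killed.
; Tick applies movement input by the MoveRight flag, which capsule hits on non-player obstacles with an X normal toggle, mirroring the sprite's X scale.
; AnyDamage lowers clamped Health, and at zero stops movement, plays the death flipbook and destroys the actor after a delay.
; An optional squash-and-tint effect is left unconnected.
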(event `self.ReceiveAnyDamage`
  (params (Damage :type "Float (single-precision)") (DamageType :type "DamageType Object Reference") (InstigatedBy :type "Controller Object Reference") (DamageCauser :type "Actor Object Reference"))
  ;[0.6344 0.343 0.3655] Enemy Health
  ;;[1 1 1] Take damage amount from health and set it between 0 and 100
  (set `self.Health` (`KismetMathLibrary.FClamp` (- (`self.Health`) Damage) 0.0 100.0))
  (if (and (<= (`self.Health`) 0.0) (not (`self.bDead`)))
    (set `self.bDead` true)
    (`self.DeathAnimation`)
    (`KismetSystemLibrary.Delay` 1.0)
    (`self.K2_DestroyActor`)))

(event `FlipSprite`
  (bind (_returnvalue_x _returnvalue_y _returnvalue_z) (`KismetMathLibrary.BreakVector` (`SceneComponent.K2_GetComponentScale` (`self.Sprite`))))
  ;[1 1 1] Flip Sprite
  (`SceneComponent.SetWorldScale3D` (`self.Sprite`) (`KismetMathLibrary.MakeVector` (* (select `bool` (`self.MoveRight`) :`false` 1.0 :`true` -1.0 :!type "Float (single-precision)") (`KismetMathLibrary.Abs` _returnvalue_x)) _returnvalue_y _returnvalue_z)))

(event `self.ReceiveTick`
  (params (DeltaSeconds :type "Float (single-precision)"))
  ;[1 1 1] Check enemy is not dead
  (if (not (`self.bDead`))
    ;[1 1 1] Add movement every tick
    (`self.AddMovementInput` (1.0 0.0 0.0) (select `bool` (`self.MoveRight`) :`false` -1.0 :`true` 1.0 :!type "Float (single-precision)"))))

(event `DeathAnimation`
  ;[1 1 1] Death Animation
  (`PaperFlipbookComponent.SetFlipbook` (`self.Sprite`) "/Game/Textures/myTextures/Deathmob1.Deathmob1"))

(event `self.CapsuleComponent.OnComponentHit`
  (params (HitComponent :type "PrimitiveComponent Object Reference") (OtherActor :type "Actor Object Reference") (OtherComp :type "PrimitiveComponent Object Reference") (NormalImpulse :type "Vector Structure") (Hit :type "HitResult Structure (by ref)"))
  ;[1 1 1] Change Direction hit wall
  (if (!= OtherActor (`GameplayStatics.GetPlayerPawn` 0))
    (if (!= (.x Hit_Normal) 0.0)
      ;;[1 1 1] Toggle boolean
      (set `self.MoveRight` (not (`self.MoveRight`)))
      ;;[0.5569 0.4157 1] Flips the sprite based on direction (double click node to see function)
      (`self.FlipSprite`))))

(fn `UserConstructionScript`)