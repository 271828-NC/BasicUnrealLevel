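; Base enemy Blueprint that handles health and death for enemies.
; AnyDamage subtracts damage from a clamped Health, and a Dead flag lets the death sequence start only once when it reaches zero.
; Death calls DeathAnimation, waits briefly, then calls EnemyDied; both functions are empty here, leaving behavior to child classes.
; An older squash-and-red-tint sprite death effect remains in the graph but is disconnected.
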(event `self.ReceiveAnyDamage`
  (params (Damage :type "Float (single-precision)") (DamageType :type "DamageType Object Reference") (InstigatedBy :type "Controller Object Reference") (DamageCauser :type "Actor Object Reference"))
  ;[0.6344 0.343 0.3655] Base Enemy Health code
  ;;[1 1 1] Take damage amount from health and set it between 0 and 100
  (set `self.Health` (`KismetMathLibrary.FClamp` (- (`self.Health`) Damage) 0.0 100.0))
  (if (and (<= (`self.Health`) 0.0) (not (`self.bDead`)))
    (set `self.bDead` true)
    (`self.DeathAnimation`)
    (`KismetSystemLibrary.Delay` 1.0)
    (`self.EnemyDied`)))

(fn `DeathAnimation`)

(fn `EnemyDied`)

(fn `UserConstructionScript`)